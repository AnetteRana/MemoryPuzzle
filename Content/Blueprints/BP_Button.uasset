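; BP_Button is a colored button that glows and plays a note chosen by its ID when clicked.
; An ID setup event stores the ID and creates a dynamic material tinted from a color array.
; Clicking passes the ID to the audio component as a note parameter and triggers visual feedback.
; The visual event optionally swaps to a squished mesh, raises emission, then restores both after a delay.
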(event Custom|ActivateButtonVisual
  (params (isPressed :type Boolean))
  ;[1 1 1] activate button visuals
  (if isPressed
    (Components|StaticMesh|SetStaticMesh (Variables|Default|GetSM_top) "/Game/Geometry/button1_squished.button1_squished"))
  (Rendering|Material|SetScalarParameterValue (Variables|Default|GetDynamicMaterial) "Param_Emission" (Variables|Default|GetGlowEmissionStrength) :!class /Script/Engine.MaterialInstanceDynamic)
  (Utilities|FlowControl|Delay (Variables|Default|GetGlowDelayTime))
  ;[1 1 1] de-activate visuals
  (if true
    (Components|StaticMesh|SetStaticMesh (Variables|Default|GetSM_top) "/Game/Geometry/button1_unsquished.button1_unsquished"))
  (Rendering|Material|SetScalarParameterValue (Variables|Default|GetDynamicMaterial) "Param_Emission" 0.0 :!class /Script/Engine.MaterialInstanceDynamic))

(event Custom|set%20ID%20and%20color
  (params (ID :type Integer))
  (Variables|Default|SetbuttonID ID)
  (bind _returnvalue (Rendering|Material|CreateDynamicMaterialInstance (Variables|Default|GetSM_top) 0 0 "None" :!class /Script/Engine.PrimitiveComponent))
  (Variables|Default|SetDynamicMaterial _returnvalue)
  (Rendering|Material|SetVectorParameterValue (Variables|Default|GetDynamicMaterial) "Param_Color" (Math|Conversions|ToLinearColor(Color) (Utilities|Array|Get(acopy) (Variables|Default|GetcolorArray) (Variables|Default|GetbuttonID))) :!class /Script/Engine.MaterialInstanceDynamic))

(event EventClicked
  ;[1 1 1] When clicked
  (CallFunction|ActivateButtonVisual true)
  (Effects|Components|ParticleSystem|SetIntParameter (Variables|Default|GetAudioNote) "NoteID" (Variables|Default|GetbuttonID))
  (Audio|Components|Audio|Play (Variables|Default|GetAudioNote) 0.0))

(fn ConstructionScript)