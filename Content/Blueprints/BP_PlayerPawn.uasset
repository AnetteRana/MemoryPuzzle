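; BP_PlayerPawn is the player pawn that handles mouse clicks on world objects and quits the game on Escape.
; A left click runs a helper that deprojects the cursor and line-traces a short distance along that direction against WorldDynamic objects, using complex collision.
; The hit actor receives ClickedMessage, so the response to a click is left to that actor.
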(event Input|MouseEvents|LeftMouseButton
  (params (Key :type Key%20Structure :default "None"))
  (:Pressed
    (bind _outhit_hitactor (|linetraceforworlddynamic_2))
    (Class|BPIClickable|Clicked(Message) _outhit_hitactor)))

(event Input|KeyboardEvents|Escape
  (params (Key :type Key%20Structure :default "None"))
  (:Pressed
    (Game|QuitGame 0 "Quit" false)))

(fn ConstructionScript)