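; Game mode for a Simon-style memory puzzle where the player repeats a random button sequence that grows by one each round.
; On StartGame it reads button and round counts from the game instance, spawns buttons in a ring, rolls the pattern and replays it with a delayed loop.
; ButtonPressed checks input, advancing rounds or showing win/lose widgets.
; Best times per button/round combination persist in a save game and supply menu score text.
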(event Custom|SpawnButtons
  ;[1 1 1] Spawn buttons
  (|setspawnlocation(basedonnumber))
  (for _index (range 0 (- (Variables|Default|GetnumberOfButtons) 1))
    (bind _returnvalue (Game|SpawnActorfromClass "/Game/Blueprints/BP_Button.BP_Button_C" (Math|Transform|MakeTransform (Math|Vector|RotateVectorAroundAxis (Variables|Default|GetSpawnLocation) (* _index (/ 3.6e+02 (Math|Conversions|ToFloat(Integer) (Variables|Default|GetnumberOfButtons)))) "0, 0,1.000000") (Math|Conversions|RotationFromXVector (Math|Vector|RotateVectorAroundAxis (Variables|Default|GetSpawnLocation) (* _index (/ 3.6e+02 (Math|Conversions|ToFloat(Integer) (Variables|Default|GetnumberOfButtons)))) "0, 0,1.000000")) "1,1,1") "Undefined" 0 0))
    (Default|GiveButtonInfo _returnvalue _index self)
    (Utilities|Array|Add (Variables|Default|GettheButtons) _returnvalue)))

(event Custom|ShowPattern
  ;[1 1 1] Show pattern
  (|HUDupdatecurrentround)
  (bind _index (Utilities|ForLoopwithDelay 0.7 0 (Variables|Default|GetcurrentRound))
    (:Loop%20Body
      (Default|ActivateButtonVisual (Utilities|Array|Get(acopy) (Variables|Default|GettheButtons) (Utilities|Array|Get(acopy) (Variables|Default|GetPattern) _index)) false))
    (:Completed
      (Variables|Default|SetisExpectingInput true)
      (Variables|/Game/UI/HUD.HUD_C|SetGMisExpectingInput (Variables|Default|GetHUD_ref) true))))

(event Custom|Check%20if%20new%20score%20is%20gooood
  (bind _foundmatchingscore (Utilities|FindPossibleMatchingScore (Variables|Default|GetnumberOfButtons) (Variables|Default|GetnumberOfRounds))
    (:Out
      (if _foundmatchingscore
        ;[1 1 1] is new time better?
        (if (< (Variables|Default|GetwinTime) (.besttime (Variables|Default|GetMatchingSavedScore)))
          ;[1 1 1] override old score
          (bind _output_get (Variables|Default|SetMatchingSavedScore (Utilities|Struct|MakeBestTimes_struct (Variables|Default|GetnumberOfButtons) (Variables|Default|GetnumberOfRounds) (Variables|Default|GetwinTime))))
          (Utilities|Array|SetArrayElem (Variables|Default|GetSaved%20Scores_GM) (Variables|Default|GetArray%20Index) _output_get)
          (Variables|/Game/Blueprints/BP_mySaveGame.BP_mySaveGame_C|SetSavedScores (Variables|Default|GetSaveGame_ref) (Variables|Default|GetSaved%20Scores_GM) :!label _label)
          (SaveGame|SaveGametoSlot (Variables|Default|GetSaveGame_ref) (Variables|Default|GetSave%20Slot%20Name)))
        (else
          (bind _output_get_2 (Variables|Default|SetMatchingSavedScore (Utilities|Struct|MakeBestTimes_struct (Variables|Default|GetnumberOfButtons) (Variables|Default|GetnumberOfRounds) (Variables|Default|GetwinTime))))
          (Utilities|Array|Add (Variables|Default|GetSaved%20Scores_GM) _output_get_2)
          (goto _label))))))

(event Custom|CreatePattern
  ;[1 1 1] Create pattern
  (for _index (range 0 (- (Variables|Default|GetnumberOfRounds) 1))
    (Utilities|Array|Insert (Variables|Default|GetPattern) (Math|Random|RandomIntegerinRange 0 (- (Variables|Default|GetnumberOfButtons) 1)) _index)))

(event Custom|StartGame
  ;[1 1 1] Start game
  (|GetnumberOfButtonsandrounds)
  (CallFunction|SpawnButtons)
  (CallFunction|CreatePattern)
  (CallFunction|ShowPattern)
  (Variables|/Game/UI/HUD.HUD_C|SettotalRounds (Variables|Default|GetHUD_ref) (Variables|Default|GetnumberOfRounds)))

(event Custom|Load%20Game
  ;[1 1 1] load saved game
  (bind _returnvalue (SaveGame|LoadGamefromSlot (Variables|Default|GetSave%20Slot%20Name)))
  (bind _asbp_my_save_game (Utilities|Casting|CastToBP_mySaveGame _returnvalue))
  (bind _output_get (Variables|Default|SetSaveGame_ref _asbp_my_save_game))
  (Variables|Default|SetSaved%20Scores_GM (Variables|/Game/Blueprints/BP_mySaveGame.BP_mySaveGame_C|GetSavedScores _output_get)))

(event Custom|ButtonPressed
  (params (buttonID :type Integer))
  ;[1 1 1] Button pressed
  ;;[1 1 1] Correct button?
  (if (== buttonID (Utilities|Array|Get(acopy) (Variables|Default|GetPattern) (Variables|Default|GetbuttonsPressedSuccessfully)))
    ;;[1 1 1] was it the last in the round?
    (if (== (Variables|Default|GetbuttonsPressedSuccessfully) (Variables|Default|GetcurrentRound))
      (bind _output_get (Variables|Default|SetcurrentRound (+ (stale _output_get) 1)))
      ;;[1 1 1] was it the last in the game?
      (if (== (Variables|Default|GetcurrentRound) (Variables|Default|GetnumberOfRounds))
        (CallFunction|GameWon)
        (else
          ;;[1 1 1] Start next round
          (Utilities|FlowControl|Delay (Variables|Default|GetDelayStartRound))
          (Variables|Default|SetisExpectingInput false)
          (Variables|/Game/UI/HUD.HUD_C|SetGMisExpectingInput (Variables|Default|GetHUD_ref) false)
          (Utilities|FlowControl|Delay (Variables|Default|GetDelayStartRound))
          (Variables|Default|SetbuttonsPressedSuccessfully 0)
          (CallFunction|ShowPattern)))
      (else
        (bind _output_get_2 (Variables|Default|SetbuttonsPressedSuccessfully (+ (stale _output_get_2) 1)))))
    (else
      (CallFunction|GameLost))))

(event Custom|Game%20won
  ;[1 1 1] Win / Lose
  (Variables|Default|SetwinTime (Utilities|Time|GetGameTimeinSeconds))
  (Utilities|Casting|CastToBP_GameInstance (Game|GetGameInstance))
  (bind _returnvalue (UserInterface|CreateWidget "/Game/UI/BPW_Win.BPW_Win_C"))
  (UserInterface|Viewport|AddtoViewport _returnvalue 0)
  (CallFunction|CheckifNewScoreIsGooood)
  (Variables|Default|SetisExpectingInput false))

(event Custom|Game%20lost
  ;[1 1 1] Win / Lose
  (Utilities|Casting|CastToBP_GameInstance (Game|GetGameInstance))
  (bind _returnvalue (UserInterface|CreateWidget "/Game/UI/BPW_Lose.BPW_Lose_C"))
  (UserInterface|Viewport|AddtoViewport _returnvalue 0)
  (Variables|Default|SetisExpectingInput false))

(event Custom|Save%20Game
  ;[1 1 1] Save object
  (Utilities|IsValid (Variables|Default|GetSaveGame_ref)
    (:Is%20Valid
      (Variables|/Game/Blueprints/BP_mySaveGame.BP_mySaveGame_C|SetSavedScores (Variables|Default|GetSaveGame_ref) (Variables|Default|GetSaved%20Scores_GM)))
    (:Is%20Not%20Valid
      (bind _returnvalue (SaveGame|CreateSaveGameObject "/Game/Blueprints/BP_mySaveGame.BP_mySaveGame_C"))
      (bind _output_get (Variables|Default|SetSaveGame_ref _returnvalue))
      (Variables|Default|SetSaved%20Scores_GM (Variables|/Game/Blueprints/BP_mySaveGame.BP_mySaveGame_C|GetSavedScores _output_get))))
  (SaveGame|SaveGametoSlot (Variables|Default|GetSaveGame_ref) (Variables|Default|GetSave%20Slot%20Name)))

(event Custom|Find%20save%20data%20matching%20buttons/levels
  ;[1 1 1] Find save data matching
  (Utilities|FindPossibleMatchingScore (Variables|Default|GetnumberOfButtons) (Variables|Default|GetnumberOfRounds)))

(event EventBeginPlay
  ;[1 1 1] Begin play - load/create save game
  (bind _returnvalue (SaveGame|DoesSaveGameExist (Variables|Default|GetSave%20Slot%20Name)))
  (if _returnvalue
    (CallFunction|LoadGame)
    (else
      (CallFunction|SaveGame))))

(fn ConstructionScript)

(fn GiveMenuScoreText
  (params (buttons :type Integer) (levels :type Integer))
  (bind _foundmatchingscore (Utilities|FindPossibleMatchingScore buttons levels)
    (:Out
      (if _foundmatchingscore
        (return (Utilities|String|Append "Best time: " (Utilities|String|ToString(Text) (Utilities|Text|ToText(Float) (.besttime (Variables|Default|GetMatchingSavedScore)) "HalfToEven" false false 1 324 0 2))))
        (else
          (return "No score yet!"))))))